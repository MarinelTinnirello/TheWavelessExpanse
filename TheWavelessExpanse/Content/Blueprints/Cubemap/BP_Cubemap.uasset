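; BP_Cubemap is a level-transition portal that sends the game to another level when its trigger box is overlapped.
; On BeginPlay it applies the configured material to the cube.
; On overlap it stores its DoorID in BP_GameInstance, then opens the level whose name comes from the Dst enum value.
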(event OnComponentBeginOverlap(TriggerBox)
  (params (OverlappedComponent :type Primitive%20Component%20Object%20Reference) (OtherActor :type Actor%20Object%20Reference) (OtherComp :type Primitive%20Component%20Object%20Reference) (OtherBodyIndex :type Integer) (bFromSweep :type Boolean) (SweepResult :type Hit%20Result%20Structure%20%28by%20ref%29))
  ;[1 1 1] Open next level
  (bind _asbp_game_instance (Utilities|Casting|CastToBP_GameInstance (Game|GetGameInstance)))
  (Variables|/Game/Blueprints/Player/BP_GameInstance.BP_GameInstance_C|SetDoorID _asbp_game_instance (Variables|Level|GetDoorID))
  (Game|OpenLevel(byName) (Utilities|String|StringToName (Utilities|String|EnumtoString (Variables|Level|GetDst)))))

(event EventBeginPlay
  ;[1 1 1] Change portal material
  (Rendering|Material|SetMaterial (Variables|Default|GetCube) 0 (Variables|Components|GetMaterial)))

(fn ConstructionScript)