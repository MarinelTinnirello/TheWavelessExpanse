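; BP_InteractablePedestal2 is a pedestal that locks an overlapping BP_Interactable in place as part of a Main Temple or Mausoleum puzzle.
; On overlap it freezes the object, swaps its material to orichalcum, turns off its own particles and snaps the object to its Scene point.
; CheckRoomForCount increments the room's GameInstance counter, revealing "ActorFire" actors and playing that room's level sequence at two or more.
; Placement state is saved to the GameInstance.
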(event OnComponentBeginOverlap(Box)
  (params (OverlappedComponent :type Primitive%20Component%20Object%20Reference) (OtherActor :type Actor%20Object%20Reference) (OtherComp :type Primitive%20Component%20Object%20Reference) (OtherBodyIndex :type Integer) (bFromSweep :type Boolean) (SweepResult :type Hit%20Result%20Structure%20%28by%20ref%29))
  (bind _gameinstref (Variables|Default|GetGameInstRef))
  (bind _scene (Variables|Default|GetScene))
  (bind _returnvalue (Transformation|GetWorldLocation _scene))
  (bind _asbp_interactable (Utilities|Casting|CastToBP_Interactable OtherActor))
  (Variables|Default|SetInteractableRef _asbp_interactable)
  (Audio|PlaySound2D "/Game/Music/SoundFX/SFX/185_-_glass.185_-_glass" 1.0 1.0 0.0 0 0)
  (Physics|SetPhysicsLinearVelocity (Variables|/Game/Blueprints/Interactable/BP_Interactable.BP_Interactable_C|GetStaticMesh (Variables|Default|GetInteractableRef)) "0, 0, 0" false "None")
  (Rendering|Material|SetMaterial (Variables|/Game/Blueprints/Interactable/BP_Interactable.BP_Interactable_C|GetStaticMesh (Variables|Default|GetInteractableRef)) 0 "/Game/Materials/Level_Assets/My_Assets/Orichalcum/MAT_Orichalcum_INST_1.MAT_Orichalcum_INST_1")
  (bind _output_get (Variables|/Game/Blueprints/Player/BP_GameInstance.BP_GameInstance_C|SetMatOnChange (Variables|Default|GetGameInstRef) "/Game/Materials/Level_Assets/My_Assets/Orichalcum/MAT_Orichalcum_INST_1.MAT_Orichalcum_INST_1"))
  (Physics|SetSimulatePhysics (Variables|/Game/Blueprints/Interactable/BP_Interactable.BP_Interactable_C|GetStaticMesh (Variables|Default|GetInteractableRef)) false)
  (Components|Activation|Deactivate (Variables|Default|GetParticleSystem))
  (bind _output_get_2 (Variables|/Game/Blueprints/Player/BP_GameInstance.BP_GameInstance_C|SetIsParticleSystemOn (Variables|Default|GetGameInstRef) false))
  (CallFunction|CheckRoomforCount (Variables|Default|GetGameInstRef) (Variables|Default|GetInteractableRef))
  (Transformation|SetActorLocation (Variables|Default|GetInteractableRef) _returnvalue false false)
  (bind _output_get_3 (Variables|/Game/Blueprints/Player/BP_GameInstance.BP_GameInstance_C|SetPlacedInteractableLoc _gameinstref _returnvalue))
  (if (Variables|/Game/Blueprints/Interactable/BP_Interactable.BP_Interactable_C|GetIsPlaced (Variables|Default|GetInteractableRef))
    (bind _output_get_4 (Variables|/Game/Blueprints/Player/BP_GameInstance.BP_GameInstance_C|SetIsPlaced _gameinstref true))
    (bind _output_get_5 (Variables|Default|SetInteractableStruct (Utilities|Struct|MakeSTRUCT_Interactable _output_get_3 _output_get _output_get_2 _output_get_4)))
    (Variables|/Game/Blueprints/Player/BP_GameInstance.BP_GameInstance_C|SetInteractableState (Variables|Default|GetGameInstRef) _output_get_5)))

(event EventBeginPlay
  (bind _asbp_game_instance (Utilities|Casting|CastToBP_GameInstance (Game|GetGameInstance)))
  (Variables|Default|SetGameInstRef _asbp_game_instance)
  (Variables|/Game/Blueprints/Player/BP_GameInstance.BP_GameInstance_C|SetInteractableState (Variables|Default|GetGameInstRef) (stale OnComponentBeginOverlap(Box) _output_get_5)))

(fn ConstructionScript)

(fn CheckRoomforCount
  (params (Game%20Instance :type BP%20Game%20Instance%20Object%20Reference) (Interactable :type BP%20Interactable%20Object%20Reference))
  (bind _interactableamt_maintemple (Variables|/Game/Blueprints/Player/BP_GameInstance.BP_GameInstance_C|GetInteractableAmt_MainTemple Game%20Instance))
  (bind _interactableamt_mausoleum (Variables|/Game/Blueprints/Player/BP_GameInstance.BP_GameInstance_C|GetInteractableAmt_Mausoleum Game%20Instance))
  (bind _ismaintemple (Variables|/Game/Blueprints/Interactable/BP_Interactable.BP_Interactable_C|GetIsMainTemple Interactable))
  (bind _ismaulsoleum (Variables|/Game/Blueprints/Interactable/BP_Interactable.BP_Interactable_C|GetIsMaulsoleum Interactable))
  (Utilities|FlowControl|Sequence
    (:then_0
      (if _ismaintemple
        (Math|Integer|IncrementInt _interactableamt_maintemple
          (:%20%20
            (if (>= _interactableamt_maintemple 2)
              (bind _outactors (Actor|GetAllActorswithTag "ActorFire" :!label _label))
              (for _array_element _outactors
                (Rendering|SetVisibility (Variables|/Script/Engine.Actor|GetRootComponent _array_element) true true))
              (Utilities|FlowControl|Sequence
                (:then_0
                  (if _ismaintemple
                    (Utilities|Casting|CastToBP_MantaRay (Game|GetPlayerCharacter 0))
                    (bind _returnvalue (Sequencer|Player|CreateLevelSequencePlayer "/Game/Animations/Cinematics/ItemDrops/MainTemple/LVSEQ_MainTemple_AddActor1.LVSEQ_MainTemple_AddActor1"))
                    (Sequencer|Player|Play _returnvalue :!class /Script/MovieScene.MovieSceneSequencePlayer)))
                (:then_1
                  (if _ismaulsoleum
                    (Utilities|Casting|CastToBP_MantaRay (Game|GetPlayerCharacter 0))
                    (bind _returnvalue_2 (Sequencer|Player|CreateLevelSequencePlayer "/Game/Animations/Cinematics/ItemDrops/Mausoleum/LVSEQ_Mausoleum_AddActor1.LVSEQ_Mausoleum_AddActor1"))
                    (Sequencer|Player|Play _returnvalue_2 :!class /Script/MovieScene.MovieSceneSequencePlayer)))))))))
    (:then_1
      (if _ismaulsoleum
        (Math|Integer|IncrementInt _interactableamt_mausoleum
          (:%20%20
            (if (>= _interactableamt_mausoleum 2)
              (goto _label))))))))