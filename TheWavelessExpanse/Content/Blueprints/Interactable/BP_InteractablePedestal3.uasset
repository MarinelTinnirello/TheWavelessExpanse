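; Pedestal that receives a BP_Interactable on box overlap, snapping it into place with physics off, an Orichalcum material, a sound and its particles switched off.
; It records the placement in BP_GameInstance, saving a state struct when the interactable is flagged as placed.
; CheckRoomForCount increments Ruins or Observatory counters, whose thresholds reveal tagged pose actors in the Ruins and play level sequences for either room, setting seen flags.
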(event OnComponentBeginOverlap(Box)
  (params (OverlappedComponent :type Primitive%20Component%20Object%20Reference) (OtherActor :type Actor%20Object%20Reference) (OtherComp :type Primitive%20Component%20Object%20Reference) (OtherBodyIndex :type Integer) (bFromSweep :type Boolean) (SweepResult :type Hit%20Result%20Structure%20%28by%20ref%29))
  (bind _gameinstref (Variables|Default|GetGameInstRef))
  (bind _scene (Variables|Default|GetScene))
  (bind _returnvalue (Transformation|GetWorldLocation _scene))
  (bind _asbp_interactable (Utilities|Casting|CastToBP_Interactable OtherActor))
  (Variables|Default|SetInteractableRef _asbp_interactable)
  (Audio|PlaySound2D "/Game/Music/SoundFX/SFX/185_-_glass.185_-_glass" 1.0 1.0 0.0 0 0)
  (Physics|SetPhysicsLinearVelocity (Variables|/Game/Blueprints/Interactable/BP_Interactable.BP_Interactable_C|GetStaticMesh (Variables|Default|GetInteractableRef)) "0, 0, 0" false "None")
  (Rendering|Material|SetMaterial (Variables|/Game/Blueprints/Interactable/BP_Interactable.BP_Interactable_C|GetStaticMesh (Variables|Default|GetInteractableRef)) 0 "/Game/Materials/Level_Assets/My_Assets/Orichalcum/MAT_Orichalcum_INST_1.MAT_Orichalcum_INST_1")
  (bind _output_get (Variables|/Game/Blueprints/Player/BP_GameInstance.BP_GameInstance_C|SetMatOnChange (Variables|Default|GetGameInstRef) "/Game/Materials/Level_Assets/My_Assets/Orichalcum/MAT_Orichalcum_INST_1.MAT_Orichalcum_INST_1"))
  (Physics|SetSimulatePhysics (Variables|/Game/Blueprints/Interactable/BP_Interactable.BP_Interactable_C|GetStaticMesh (Variables|Default|GetInteractableRef)) false)
  (Components|Activation|Deactivate (Variables|Default|GetParticleSystem))
  (bind _output_get_2 (Variables|/Game/Blueprints/Player/BP_GameInstance.BP_GameInstance_C|SetIsParticleSystemOn (Variables|Default|GetGameInstRef) false))
  (CallFunction|CheckRoomforCount (Variables|Default|GetGameInstRef) (Variables|Default|GetInteractableRef))
  (Transformation|SetActorLocation (Variables|Default|GetInteractableRef) _returnvalue false false)
  (bind _output_get_3 (Variables|/Game/Blueprints/Player/BP_GameInstance.BP_GameInstance_C|SetPlacedInteractableLoc _gameinstref _returnvalue))
  (if (Variables|/Game/Blueprints/Interactable/BP_Interactable.BP_Interactable_C|GetIsPlaced (Variables|Default|GetInteractableRef))
    (bind _output_get_4 (Variables|/Game/Blueprints/Player/BP_GameInstance.BP_GameInstance_C|SetIsPlaced _gameinstref true))
    (bind _output_get_5 (Variables|Default|SetInteractableStruct (Utilities|Struct|MakeSTRUCT_Interactable _output_get_3 _output_get _output_get_2 _output_get_4)))
    (Variables|/Game/Blueprints/Player/BP_GameInstance.BP_GameInstance_C|SetInteractableState (Variables|Default|GetGameInstRef) _output_get_5)))

(event EventBeginPlay
  (bind _asbp_game_instance (Utilities|Casting|CastToBP_GameInstance (Game|GetGameInstance)))
  (Variables|Default|SetGameInstRef _asbp_game_instance)
  (Variables|/Game/Blueprints/Player/BP_GameInstance.BP_GameInstance_C|SetInteractableState (Variables|Default|GetGameInstRef) (stale OnComponentBeginOverlap(Box) _output_get_5)))

(fn ConstructionScript)

(fn CheckRoomforCount
  (params (Game%20Instance :type BP%20Game%20Instance%20Object%20Reference) (Interactable :type BP%20Interactable%20Object%20Reference))
  (bind _interactableamt_observatory (Variables|/Game/Blueprints/Player/BP_GameInstance.BP_GameInstance_C|GetInteractableAmt_Observatory Game%20Instance))
  (bind _interactableamt_ruins (Variables|/Game/Blueprints/Player/BP_GameInstance.BP_GameInstance_C|GetInteractableAmt_Ruins Game%20Instance))
  (Utilities|FlowControl|Sequence
    (:then_0
      (if (Variables|/Game/Blueprints/Interactable/BP_Interactable.BP_Interactable_C|GetIsRuins Interactable)
        (Math|Integer|IncrementInt _interactableamt_ruins
          (:%20%20
            (if (>= _interactableamt_ruins 1)
              (bind _outactors (Actor|GetAllActorswithTag "ActorPose1"))
              (for _array_element _outactors
                (Rendering|SetVisibility (Variables|/Script/Engine.Actor|GetRootComponent _array_element) true true)
                (Collision|SetActorEnableCollision _array_element false)
                (if (>= _interactableamt_ruins 2)
                  (bind _outactors_2 (Actor|GetAllActorswithTag "ActorPose2"))
                  (for _array_element_2 _outactors_2
                    (Rendering|SetVisibility (Variables|/Script/Engine.Actor|GetRootComponent _array_element_2) true true)
                    (Collision|SetActorEnableCollision _array_element_2 false))
                  (Utilities|Casting|CastToBP_MantaRay (Game|GetPlayerCharacter 0))
                  (bind _returnvalue (Sequencer|Player|CreateLevelSequencePlayer "/Game/Animations/Cinematics/ItemDrops/Ruins/LVSEQ_Ruins_AddActor2.LVSEQ_Ruins_AddActor2"))
                  (Sequencer|Player|Play _returnvalue :!class /Script/MovieScene.MovieSceneSequencePlayer)
                  (Variables|/Game/Blueprints/Player/BP_GameInstance.BP_GameInstance_C|SetHasSeenRuins (Variables|Default|GetGameInstRef) true)))
              (Utilities|Casting|CastToBP_MantaRay (Game|GetPlayerCharacter 0))
              (bind _returnvalue_2 (Sequencer|Player|CreateLevelSequencePlayer "/Game/Animations/Cinematics/ItemDrops/Ruins/LVSEQ_Ruins_AddActor1.LVSEQ_Ruins_AddActor1"))
              (Sequencer|Player|Play _returnvalue_2 :!class /Script/MovieScene.MovieSceneSequencePlayer)
              (if (>= _interactableamt_ruins 2)
                (bind _outactors_3 (Actor|GetAllActorswithTag "ActorPose2"))
                (for _array_element_3 _outactors_3
                  (Rendering|SetVisibility (Variables|/Script/Engine.Actor|GetRootComponent _array_element_3) true true)
                  (Collision|SetActorEnableCollision _array_element_3 false))
                (Utilities|Casting|CastToBP_MantaRay (Game|GetPlayerCharacter 0))
                (bind _returnvalue_3 (Sequencer|Player|CreateLevelSequencePlayer "/Game/Animations/Cinematics/ItemDrops/Ruins/LVSEQ_Ruins_AddActor2.LVSEQ_Ruins_AddActor2"))
                (Sequencer|Player|Play _returnvalue_3 :!class /Script/MovieScene.MovieSceneSequencePlayer)
                (Variables|/Game/Blueprints/Player/BP_GameInstance.BP_GameInstance_C|SetHasSeenRuins (Variables|Default|GetGameInstRef) true)))))))
    (:then_1
      (if (Variables|/Game/Blueprints/Interactable/BP_Interactable.BP_Interactable_C|GetIsObservatory Interactable)
        (Math|Integer|IncrementInt _interactableamt_observatory
          (:%20%20
            (if (>= _interactableamt_observatory 2)
              (bind _asbp_manta_ray (Utilities|Casting|CastToBP_MantaRay (Game|GetPlayerCharacter 0)))
              (Variables|/Game/Blueprints/Player/BP_MantaRay.BP_MantaRay_C|SetIsMovable _asbp_manta_ray false)
              (bind _returnvalue_4 (Sequencer|Player|CreateLevelSequencePlayer "/Game/Animations/Cinematics/Cutscenes/LVLSEQ_ObservatoryEvent.LVLSEQ_ObservatoryEvent"))
              (Sequencer|Player|Play _returnvalue_4 :!class /Script/MovieScene.MovieSceneSequencePlayer)
              (Variables|/Game/Blueprints/Player/BP_MantaRay.BP_MantaRay_C|SetIsMovable _asbp_manta_ray true)
              (bind _asbp_game_instance (Utilities|Casting|CastToBP_GameInstance (Game|GetGameInstance)))
              (Variables|/Game/Blueprints/Player/BP_GameInstance.BP_GameInstance_C|SetHasSeenCutscene _asbp_game_instance true))))))))