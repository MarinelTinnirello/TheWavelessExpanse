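; BP_DemonFish is an enemy fish that switches to swimming movement on BeginPlay and records its spawn location.
; Each Tick it adds a small random yaw to DemonFishEyecosphere, giving an uneven spin.
; RotateActorAroundPoint places an actor on a horizontal circle around a target actor or fallback location.
; The orbit logic using it, with direction and debug-line options, is disconnected, so the fish does not orbit.
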(event EventBeginPlay
  (Pawn|Components|CharacterMovement|SetMovementMode (Variables|Character|GetCharacterMovement) "MOVE_Swimming" 0)
  (Variables|RotateActorAroundPoint|SetInitLoc (Transformation|GetActorLocation)))

(event Collision|EventActorBeginOverlap
  (params (OtherActor :type Actor%20Object%20Reference)))

(event EventTick
  (params (DeltaSeconds :type Float%20%28single-precision%29))
  (Transformation|AddLocalRotation (Variables|Default|GetDemonFish_Eyecosphere) (Math|Rotator|MakeRotator 0.0 0.0 (Math|Random|RandomFloatinRange 0.0 5.0)) false false))

(fn ConstructionScript)

(fn RotateActorAroundPoint
  (params (Actor :type Actor%20Object%20Reference) (Target :type Actor%20Object%20Reference) (TargetLoc :type Vector) (Radius :type Float%20%28single-precision%29) (Angle :type Float%20%28single-precision%29) (RotRate :type Float%20%28single-precision%29))
  (LocalVariables|SetL_Actor Actor)
  (LocalVariables|SetL_Target Target)
  (LocalVariables|SetL_TargetLoc TargetLoc)
  (LocalVariables|SetL_Radius Radius)
  (LocalVariables|SetL_Angle Angle)
  (LocalVariables|SetL_RotRate RotRate)
  (Utilities|IsValid (LocalVariables|GetL_Target)
    (:Is%20Valid
      (LocalVariables|SetL_TargetLoc (Transformation|GetActorLocation (LocalVariables|GetL_Target))))
    (:Is%20Not%20Valid
      _))
  (Transformation|SetActorLocation (LocalVariables|GetL_Actor) (+ (LocalVariables|GetL_TargetLoc) (Math|Vector|RotateVectorAroundAxis (Math|Vector|MakeVector (LocalVariables|GetL_Radius) 0.0 0.0) (+ (LocalVariables|GetL_RotRate) (LocalVariables|GetL_Angle)) "0, 0,1.000000")) false false)
  (return (LocalVariables|GetL_TargetLoc)))