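; BP_AnimationTrigger is a trigger volume that reveals animation actors while the BP_MantaRay is inside its Box.
; Begin overlap makes every actor tagged ActorAnim visible, including child components, and disables their collision.
; End overlap hides them again without restoring collision, and both events play the Save_Point sound attached to the overlapping component.
; An unconnected leftover branch would call MoveCharacter on every BP_WalkSpline_Character but never runs.
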(event OnComponentBeginOverlap(Box)
  (params (OverlappedComponent :type Primitive%20Component%20Object%20Reference) (OtherActor :type Actor%20Object%20Reference) (OtherComp :type Primitive%20Component%20Object%20Reference) (OtherBodyIndex :type Integer) (bFromSweep :type Boolean) (SweepResult :type Hit%20Result%20Structure%20%28by%20ref%29))
  (Utilities|Casting|CastToBP_MantaRay OtherActor)
  (bind _outactors (Actor|GetAllActorswithTag "ActorAnim"))
  (for _array_element _outactors
    (Rendering|SetVisibility (Variables|/Script/Engine.Actor|GetRootComponent _array_element) true true)
    (Collision|SetActorEnableCollision _array_element false))
  (Audio|SpawnSoundAttached "/Game/Music/SoundFX/SFX/Save_Point.Save_Point" OtherComp "None" "0, 0, 0" "0, 0, 0" "KeepRelativeOffset" false 1.0 1.0 0.0 0 0))

(event OnComponentEndOverlap(Box)
  (params (OverlappedComponent :type Primitive%20Component%20Object%20Reference) (OtherActor :type Actor%20Object%20Reference) (OtherComp :type Primitive%20Component%20Object%20Reference) (OtherBodyIndex :type Integer))
  (Utilities|Casting|CastToBP_MantaRay OtherActor)
  (bind _outactors (Actor|GetAllActorswithTag "ActorAnim"))
  (for _array_element _outactors
    (Rendering|SetVisibility (Variables|/Script/Engine.Actor|GetRootComponent _array_element) false true))
  (Audio|SpawnSoundAttached "/Game/Music/SoundFX/SFX/Save_Point.Save_Point" OtherComp "None" "0, 0, 0" "0, 0, 0" "KeepRelativeOffset" false 1.0 1.0 0.0 0 0))

(fn ConstructionScript)