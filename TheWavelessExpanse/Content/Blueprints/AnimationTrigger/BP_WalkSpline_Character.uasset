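; Character actor that travels along a referenced spline track, playing a looping walk or run animation.
; MoveCharacter picks the animation from IsWalker, then plays a timeline scaled to Duration from a configurable start offset.
; Each update maps the timeline alpha to a distance along the spline and sets the actor's world location and rotation to match.
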(event Custom|Move%20Character
  (bind _splinetrack (Variables|WalkTrack|GetSplineTrack))
  (bind _skeletalmesh (Variables|Default|GetSkeletalMesh))
  (bind _track (Variables|Default|GetTrack))
  (bind _spline (Variables|/Game/Blueprints/AnimationTrigger/BP_WalkSpline.BP_WalkSpline_C|GetSpline _splinetrack))
  (if (Variables|Default|GetIsWalker)
    (Components|Animation|PlayAnimation _skeletalmesh "/Game/ThirdPerson/Mannequin/Animations/ThirdPersonWalk.ThirdPersonWalk" true)
    (else
      (Components|Animation|PlayAnimation _skeletalmesh "/Game/ThirdPerson/Mannequin/Animations/ThirdPersonRun.ThirdPersonRun" true)))
  (Components|Timeline|SetPlayRate _track (/ 1.0 (Variables|WalkTrack|GetDuration)))
  (Components|Timeline|SetNewTime _track (Variables|WalkTrack|GetActorStartOffset))
  (bind _alpha (Timeline|Track Play)
    (:Update
      (Variables|WalkTrack|SetAlpha _alpha)
      (Transformation|SetActorLocationAndRotation (Spline|GetLocationatDistanceAlongSpline _spline (Math|Float|Lerp 0.0 (Spline|GetSplineLength _spline) (Variables|WalkTrack|GetAlpha)) "World") (Spline|GetRotationatDistanceAlongSpline _spline (Math|Float|Lerp 0.0 (Spline|GetSplineLength _spline) (Variables|WalkTrack|GetAlpha)) "World")))))

(fn ConstructionScript)