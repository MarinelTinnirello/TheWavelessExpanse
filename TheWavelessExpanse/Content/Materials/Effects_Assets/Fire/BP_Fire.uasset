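; BP_Fire is a fire effect actor that combines a material-driven static mesh with a flickering point light.
; On BeginPlay, the Flickering timeline scales the light by Intensity and reapplies Material to the mesh on each update.
; A looping timer calls GetAngle every tenth of a second to billboard the whole actor toward the player camera, flattened to horizontal so it only yaws.
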(event EventBeginPlay
  (Utilities|Time|SetTimerbyFunctionName 0 "GetAngle" 0.1 true)
  (bind _flickering (Timeline|Flickering Play)
    (:Update
      (Rendering|Components|Light|SetIntensity (Variables|Default|GetPointLight) (* _flickering (Variables|Default|GetIntensity)))
      (Rendering|Material|SetMaterial (Variables|Default|GetStaticMesh) 0 (Variables|Default|GetMaterial)))))

(fn ConstructionScript)

(fn GetAngle
  (Transformation|SetActorRotation (Math|Rotator|MakeRotfromX (Math|Vector|Normalize (* (- (Camera|GetCameraLocation (Game|GetPlayerCameraManager 0)) (Transformation|GetActorLocation)) "1.000000,1.000000,0.000000")))))